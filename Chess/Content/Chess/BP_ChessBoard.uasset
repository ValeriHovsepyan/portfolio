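; Chess board actor that lays out an 8x8 checkerboard and turns it into individual tile actors at play time.
; The construction script builds a black-and-white grid of static mesh components, hidden in game, as a layout template.
; BeginPlay enables click events, caches the player character and spawns a BP_OnePeaceOfBoard with matching material at each template transform.
; SetIntensity, not called here, alternates tile light intensity by array index parity.
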(event `self.ReceiveBeginPlay`
  (set `PlayerController.bEnableClickEvents` true (`GameplayStatics.GetPlayerController` 0))
  (bind _asbp_third_person_character (cast `/Game/ThirdPerson/Blueprints/BP_ThirdPersonCharacter` (`GameplayStatics.GetPlayerCharacter` 0)))
  (set `self.Character` _asbp_third_person_character)
  (`self.MyConstructionScript`))

(fn `MyConstructionScript`
  (for _index (range 64)
    (bind _returnvalue (`SceneComponent.K2_GetComponentToWorld` (`|GetArrayItem` (`self.BoardArray`) _index)))
    (bind _returnvalue_2 (`|SpawnActorFromClass` "/Game/Chess/BP_OnePeaceOfBoard.BP_OnePeaceOfBoard_C" _returnvalue "Undefined" "MultiplyWithRoot" null null))
    (bind _mesh (`OnePeaceOfBoard.Mesh` _returnvalue_2))
    (`SceneComponent.K2_SetWorldTransform` _mesh _returnvalue false false)
    (`PrimitiveComponent.SetMaterial` _mesh 0 (select `bool` (xor (`KismetMathLibrary.Conv_IntToBool` (mod _index 2)) (`KismetMathLibrary.Conv_IntToBool` (mod (/ _index 8) 2))) :`false` "/Game/Chess/M_BlackBoard.M_BlackBoard" :`true` "/Game/Chess/M_WhiteBoard.M_WhiteBoard" :!type "Material Object Reference"))))

(fn `SetIntensity`
  (bind _outactors (`GameplayStatics.GetAllActorsOfClass` "/Game/Chess/BP_OnePeaceOfBoard.BP_OnePeaceOfBoard_C"))
  (for (_array_element _array_index) _outactors
    (if (== (mod _array_index 2) 0)
      (bind _light (`OnePeaceOfBoard.Light` _array_element))
      (`LightComponent.SetIntensity` _light 2500000.0)
      (else
        (`LightComponent.SetIntensity` _light 1500000.0)))))

(fn `UserConstructionScript`
  (for _index (range 64)
    (bind _returnvalue (`AddComponent|NODE_AddStaticMeshComponent-0` :`RelativeTransform` (`KismetMathLibrary.Conv_VectorToTransform` (`KismetMathLibrary.MakeVector` (* (/ _index 8) 1000.0) (* (mod _index 8) 1000.0)))))
    (`SceneComponent.SetHiddenInGame` _returnvalue true false)
    (`PrimitiveComponent.SetMaterial` _returnvalue 0 (select `bool` (xor (`KismetMathLibrary.Conv_IntToBool` (mod _index 2)) (`KismetMathLibrary.Conv_IntToBool` (mod (/ _index 8) 2))) :`false` "/Game/Chess/M_BlackBoard.M_BlackBoard" :`true` "/Game/Chess/M_WhiteBoard.M_WhiteBoard" :!type "Material Object Reference"))
    (`KismetArrayLibrary.Array_Add` (`self.BoardArray`) _returnvalue)))
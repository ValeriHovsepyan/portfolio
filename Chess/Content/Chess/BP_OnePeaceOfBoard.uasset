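; BP_OnePeaceOfBoard is a clickable chess board square that moves the selected piece onto itself.
; On BeginPlay it enables click events, caches the BP_ThirdPersonCharacter and snaps the first actor overlapping its Box to the square's XY.
; A mesh click moves the character's WhiteCoin, or otherwise BlackCoin, here and turns off its location markers.
; After a successful move it increments rounds, then following a short delay changes camera and clears the selection.
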(event `self.ReceiveBeginPlay`
  (bind (_returnvalue_x _returnvalue_y) (`KismetMathLibrary.BreakVector` (`SceneComponent.K2_GetComponentLocation` (`self.Mesh`))))
  (bind _output (`|GetArrayItem` (`PrimitiveComponent.GetOverlappingActors` (`self.Box`) null)))
  (bind (_returnvalue_x_2 _returnvalue_y_2 _returnvalue_z) (`KismetMathLibrary.BreakVector` (`self.K2_GetActorLocation` _output)))
  (set `PlayerController.bEnableClickEvents` true (`GameplayStatics.GetPlayerController` 0))
  (bind _asbp_third_person_character (cast `/Game/ThirdPerson/Blueprints/BP_ThirdPersonCharacter` (`GameplayStatics.GetPlayerCharacter` 0)))
  (set `self.Character` _asbp_third_person_character)
  (`/Engine/EditorBlueprintResources/StandardMacros.IsValid` _output
    (:`Is Valid`
      (`self.K2_SetActorLocation` _output (`KismetMathLibrary.MakeVector` _returnvalue_x _returnvalue_y _returnvalue_z) false false))))

(event `self.Mesh.OnClicked`
  (params (TouchedComponent :type "PrimitiveComponent Object Reference") (ButtonPressed :type "Key Structure"))
  (bind _character (`self.Character`))
  (bind (_returnvalue_x _returnvalue_y) (`KismetMathLibrary.BreakVector` (`SceneComponent.K2_GetComponentLocation` (`self.Mesh`))))
  (bind _whitecoin (`/Game/ThirdPerson/Blueprints/BP_ThirdPersonCharacter.WhiteCoin` _character)
    (:`then`
      (bind (_returnvalue_x_2 _returnvalue_y_2 _returnvalue_z) (`KismetMathLibrary.BreakVector` (`self.K2_GetActorLocation` _whitecoin)))
      (`WhiteChessFigure.move` _whitecoin (`KismetMathLibrary.MakeVector` _returnvalue_x _returnvalue_y _returnvalue_z))
      (`WhiteChessFigure.TurnOffLocations` _whitecoin)
      (if (`WhiteChessFigure.moved` _whitecoin)
        (`ChessCharacter.IncrementRounds` _character)
        (if (`WhiteChessFigure.moved` _whitecoin)
          (set `WhiteChessFigure.moved` false _whitecoin)
          (`KismetSystemLibrary.Delay` 0.3)
          (`/Game/ThirdPerson/Blueprints/BP_ThirdPersonCharacter.ChangeCamera` _character)
          (set `/Game/ThirdPerson/Blueprints/BP_ThirdPersonCharacter.WhiteCoin` null _character))))
    (:`else`
      (bind _blackcoin (`/Game/ThirdPerson/Blueprints/BP_ThirdPersonCharacter.BlackCoin` _character)
        (:`then`
          (bind (_returnvalue_x_3 _returnvalue_y_3 _returnvalue_z_2) (`KismetMathLibrary.BreakVector` (`self.K2_GetActorLocation` _blackcoin)))
          (`BlackChessFigure.move` _blackcoin (`KismetMathLibrary.MakeVector` _returnvalue_x _returnvalue_y _returnvalue_z_2))
          (`BlackChessFigure.TurnOffLocations` _blackcoin)
          (if (`BlackChessFigure.moved` _blackcoin)
            (`ChessCharacter.IncrementRounds` _character)
            (if (`BlackChessFigure.moved` _blackcoin)
              (set `BlackChessFigure.moved` false _blackcoin)
              (`KismetSystemLibrary.Delay` 0.3)
              (`/Game/ThirdPerson/Blueprints/BP_ThirdPersonCharacter.ChangeCamera` _character)
              (set `/Game/ThirdPerson/Blueprints/BP_ThirdPersonCharacter.BlackCoin` null _character))))
        (:`else`)))))

(fn `UserConstructionScript`)
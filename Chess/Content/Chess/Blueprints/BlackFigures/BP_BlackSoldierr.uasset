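; Black soldier (pawn) piece for a chess game, handling click selection and capture.
; At startup it caches the player character and black king, creates a figure-change widget and triggers a camera change.
; On odd rounds a click restores the previous selection's material, runs a check test, shows move locations and highlights itself.
; On even rounds the selected white piece attacks it; a successful move advances the round, switches camera and destroys it.
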(event `self.ReceiveBeginPlay`
  (set `PlayerController.bEnableClickEvents` true (`GameplayStatics.GetPlayerController` 0))
  (bind _asbp_third_person_character (cast `/Game/ThirdPerson/Blueprints/BP_ThirdPersonCharacter` (`GameplayStatics.GetPlayerCharacter` 0)))
  (bind _output_get (set `self.Character` _asbp_third_person_character))
  (bind _outactors (`GameplayStatics.GetAllActorsOfClass` "/Game/Chess/Blueprints/BlackFigures/BP_BlackKing.BP_BlackKing_C"))
  (set `self.BlackKing` (`|GetArrayItem` _outactors))
  (bind _returnvalue (`|CreateWidget` "/Game/Chess/UserInterface/WBP_BlackSoldierChangeFigure.WBP_BlackSoldierChangeFigure_C"))
  (set `self.ChangeSoldierRef` _returnvalue)
  (`/Game/ThirdPerson/Blueprints/BP_ThirdPersonCharacter.ChangeCamera` _output_get))

(event `self.Mesh.OnClicked`
  (params (TouchedComponent :type "PrimitiveComponent Object Reference") (ButtonPressed :type "Key Structure"))
  (if (== (mod (`ChessCharacter.NumberOfRounds` (`self.Character`)) 2) 1)
    (`self.TurnOffLocations`)
    (bind _character (`self.Character`)
      (:`then`
        (bind _blackcoin (`/Game/ThirdPerson/Blueprints/BP_ThirdPersonCharacter.BlackCoin` _character)
          (:`then`
            (`self.TurnOffLocations`)
            (`PrimitiveComponent.SetMaterial` (`BlackChessFigure.Mesh` _blackcoin) 0 (`BlackChessFigure.Material` _blackcoin)))
          (:`else`
            _))
        (`self.WillOpenChack`)
        (`self.ShowLocations`)
        (`PrimitiveComponent.SetMaterial` (`self.Mesh`) 0 "/AnimationSharing/AnimSharingRed.AnimSharingRed")
        (set `/Game/ThirdPerson/Blueprints/BP_ThirdPersonCharacter.BlackCoin` self (`self.Character`)))
      (:`else`))
    (else
      (bind _whitecoin (`/Game/ThirdPerson/Blueprints/BP_ThirdPersonCharacter.WhiteCoin` _character)
        (:`then`
          (`WhiteChessFigure.Attack` _whitecoin self)
          (if (`WhiteChessFigure.moved` _whitecoin)
            (set `WhiteChessFigure.moved` false _whitecoin)
            (set `/Game/ThirdPerson/Blueprints/BP_ThirdPersonCharacter.WhiteCoin` null _character)
            (`ChessCharacter.IncrementRounds` _character)
            (`KismetSystemLibrary.Delay` 0.2)
            (`/Game/ThirdPerson/Blueprints/BP_ThirdPersonCharacter.ChangeCamera` _character)
            (`self.K2_DestroyActor`)))
        (:`else`)))))

(fn `UserConstructionScript`)
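; BP_WhiteQuin is the white queen piece in a chess game, handling selection and capture through mesh clicks.
; On white's turn, set by round parity on the player character, a click clears the previous selection, calls WillOpenChack and ShowLocations, then highlights itself as the selected piece.
; On black's turn, a click lets the selected black piece attack it, advancing the round and switching camera if that piece moved.
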(event `self.ReceiveBeginPlay`
  (set `PlayerController.bEnableClickEvents` true (`GameplayStatics.GetPlayerController` 0))
  (bind _asbp_third_person_character (cast `/Game/ThirdPerson/Blueprints/BP_ThirdPersonCharacter` (`GameplayStatics.GetPlayerCharacter` 0)))
  (set `self.Character` _asbp_third_person_character)
  (bind _outactors (`GameplayStatics.GetAllActorsOfClass` "/Game/Chess/Blueprints/WhiteFigures/BP_WhiteKing.BP_WhiteKing_C"))
  (set `self.WhiteKing` (`|GetArrayItem` _outactors)))

(event `self.Mesh.OnClicked`
  (params (TouchedComponent :type "PrimitiveComponent Object Reference") (ButtonPressed :type "Key Structure"))
  (bind _character (`self.Character`))
  (if (== (mod (`ChessCharacter.NumberOfRounds` (`self.Character`)) 2) 0)
    (`self.TurnOffLocations`)
    (bind _whitecoin (`/Game/ThirdPerson/Blueprints/BP_ThirdPersonCharacter.WhiteCoin` _character)
      (:`then`
        (`self.TurnOffLocations`)
        (`PrimitiveComponent.SetMaterial` (`WhiteChessFigure.Mesh` _whitecoin) 0 (`WhiteChessFigure.Material` _whitecoin))
        (set `/Game/ThirdPerson/Blueprints/BP_ThirdPersonCharacter.WhiteCoin` null _character))
      (:`else`
        _))
    (`self.WillOpenChack`)
    (`self.ShowLocations`)
    (`PrimitiveComponent.SetMaterial` (`self.Mesh`) 0 "/AnimationSharing/AnimSharingRed.AnimSharingRed")
    (set `/Game/ThirdPerson/Blueprints/BP_ThirdPersonCharacter.WhiteCoin` self (`self.Character`))
    (else
      (bind _blackcoin (`/Game/ThirdPerson/Blueprints/BP_ThirdPersonCharacter.BlackCoin` _character)
        (:`then`
          (`BlackChessFigure.Attack` _blackcoin self)
          (if (`BlackChessFigure.moved` _blackcoin)
            (set `BlackChessFigure.moved` false _blackcoin)
            (set `/Game/ThirdPerson/Blueprints/BP_ThirdPersonCharacter.WhiteCoin` null _character)
            (`ChessCharacter.IncrementRounds` _character)
            (`KismetSystemLibrary.Delay` 0.2)
            (`/Game/ThirdPerson/Blueprints/BP_ThirdPersonCharacter.ChangeCamera` _character)))
        (:`else`)))))

(fn `UserConstructionScript`)
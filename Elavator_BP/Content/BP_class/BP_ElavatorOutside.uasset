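; BP_ElavatorOutside is an outside elevator call panel with clickable up and down elements.
; On BeginPlay it enables click events on the first player controller.
; Clicking either element calls Move on a referenced Lift with this panel's FloorNum; the up click also prints the floor number plus one.
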(event `self.ReceiveBeginPlay`
  (set `PlayerController.bEnableClickEvents` true (`GameplayStatics.GetPlayerController` 0)))

(event `self.Elavator UP.OnClicked`
  (params (TouchedComponent :type "PrimitiveComponent Object Reference") (ButtonPressed :type "Key Structure"))
  (bind _floor_num (`self.floor num`))
  (`/Game/BP_class/BP_Lift.move` (`self.lift`) _floor_num)
  (`KismetSystemLibrary.PrintString` (`KismetStringLibrary.Conv_IntToString` (+ _floor_num 1))))

(event `self.Elavator Down.OnClicked`
  (params (TouchedComponent :type "PrimitiveComponent Object Reference") (ButtonPressed :type "Key Structure"))
  (`/Game/BP_class/BP_Lift.move` (`self.lift`) (`self.floor num`)))

(fn `UserConstructionScript`)
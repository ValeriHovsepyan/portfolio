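; BP_Button is a clickable lift floor button that sends a referenced Lift to its assigned floor.
; On BeginPlay, its TextRender label shows the zero-based FloorToGoButton index plus one.
; Clicking the Button component closes the lift door, waits through a fixed delay, calls Move with that index, then prints the displayed floor number.
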(event `self.ReceiveBeginPlay`
  (`TextRenderComponent.K2_SetText` (`self.TextRender`) (`KismetTextLibrary.Conv_StringToText` (`KismetStringLibrary.Conv_IntToString` (+ (`self.Floor to go button`) 1)))))

(event `self.Button.OnClicked`
  (params (TouchedComponent :type "PrimitiveComponent Object Reference") (ButtonPressed :type "Key Structure"))
  (bind _lift (`self.Lift`))
  (bind _floor_to_go_button (`self.Floor to go button`))
  (`/Game/BP_class/BP_Lift.CloseDoor` _lift)
  (`KismetSystemLibrary.Delay` 2.0)
  (`/Game/BP_class/BP_Lift.move` _lift _floor_to_go_button)
  (`KismetSystemLibrary.PrintString` (`KismetStringLibrary.Conv_IntToString` (+ _floor_to_go_button 1))))

(fn `UserConstructionScript`)
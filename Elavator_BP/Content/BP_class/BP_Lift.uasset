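; Multi-floor elevator actor that carries its cab between floors and swings its door open on arrival.
; Construction script lays out static meshes for shaft sections and a button grid; BeginPlay spawns the matching BP_ElavatorOutside and BP_Button actors, attaching buttons to the cab.
; Move sets the target height and travel time only while the door is closed.
; Timelines lerp cab location and door rotation, with delays before automatic closing.
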(event `self.ReceiveBeginPlay`
  ;[1 1 1] Event Begin play
  (`|ExecutionSequence`
    (:`then_0`
      (set `PlayerController.bShowMouseCursor` true (`GameplayStatics.GetPlayerController` 0))
      (`self.My Construction script`))
    (:`then_1`
      (set `self.Height of floor` (`self.end location`)))
    (:`then_2`
      (set `self.start location` (`SceneComponent.RelativeLocation` (`self.Elavator`))))))

(event `forward`
  ;[1 1 1] Forward
  (`TimelineComponent.SetPlayRate` (`self.tm_movement`) (/ 1.0 (`self.time`)))
  (if (!= (`self.end location`) (`self.start location`))
    (bind (_direction _alpha) (`Timeline|tm_movement` :!via `PlayFromStart`)
      (:`Update`
        (`SceneComponent.K2_SetRelativeLocation` (`self.Elavator`) (`KismetMathLibrary.VLerp` (`self.start location`) (`self.end location`) _alpha) false false))
      (:`Finished`
        (set `self.start location` (`self.end location`))
        (`KismetSystemLibrary.Delay` 1.0)
        (`self.OpenDoor`)
        (`KismetSystemLibrary.Delay` 3.0)
        (`self.CloseDoor`)))
    (else
      (`self.OpenDoor`))))

(event `OpenDoor`
  ;[1 1 1] Open door
  (if (not (`self.DoorIsOpen`))
    (bind (_direction _newtrack_0) (`Timeline|tm_OpenDoor` :!via `PlayFromStart`)
      (:`Update`
        (`SceneComponent.K2_SetRelativeRotation` (`self.elevator3_door`) (`KismetMathLibrary.RLerp` (struct) (struct :`Yaw` -90.0) _newtrack_0) false false))
      (:`Finished`
        (set `self.DoorIsOpen` true)
        (`KismetSystemLibrary.Delay` 3.0)
        (`self.CloseDoor`)))))

(event `CloseDoor`
  ;[1 1 1] Close door
  (if (`self.DoorIsOpen`)
    (bind (_direction _newtrack_0) (`Timeline|tm_closeDoor` :!via `PlayFromStart`)
      (:`Update`
        (`SceneComponent.K2_SetRelativeRotation` (`self.elevator3_door`) (`KismetMathLibrary.RLerp` (struct :`Yaw` -90.0) (struct) _newtrack_0) false false)
        (set `self.DoorIsOpen` false)))))

(fn `move`
  (params (floor :type Integer))
  (locals (`Floor move` :type Integer))
  (bind (_end_location_x _end_location_y _end_location_z) (`KismetMathLibrary.BreakVector` (`self.end location`)))
  (bind (_start_location_x _start_location_y _start_location_z) (`KismetMathLibrary.BreakVector` (`self.start location`)))
  (bind (_height_of_floor_x _height_of_floor_y _height_of_floor_z) (`KismetMathLibrary.BreakVector` (`self.Height of floor`)))
  (if (not (`self.DoorIsOpen`))
    (set `self.end location` (+ (`self.Height of floor`) (`KismetMathLibrary.MakeVector` 0.0 0.0 (* (- floor 1) (`self.Height of ElavatorOutside`)))))
    (set `self.time` (* (/ (`KismetMathLibrary.Abs` (- _end_location_z _start_location_z)) _height_of_floor_z) (`self.Duration`)))
    (`self.forward`)))

(fn `My Construction script`
  (bind _count (`self.Count`))
  (bind (_returnvalue_x _returnvalue_y) (`KismetMathLibrary.BreakVector` (`SceneComponent.K2_GetComponentLocation` (`self.Elavator`))))
  (bind (_returnvalue_x_2 _returnvalue_y_2 _returnvalue_z) (`KismetMathLibrary.BreakVector` (`SceneComponent.K2_GetComponentLocation` (`self.Button place`))))
  (`|ExecutionSequence`
    (:`then_0`
      ;[1 1 1] Elavator Outside
      (for _index (range (+ (`self.Number Of Floors`) 1))
        (bind (_intvector_x _intvector_y _intvector_z) (break `IntVector` (make `IntVector` 0 0 (* _index (`self.Height of ElavatorOutside`)))))
        (bind _returnvalue_location (`KismetMathLibrary.BreakTransform` (`KismetMathLibrary.MakeTransform` (`KismetMathLibrary.MakeVector` _returnvalue_x _returnvalue_y (+ (`KismetMathLibrary.Conv_IntToDouble` _intvector_z) 0.05)))))
        (bind _returnvalue (`|SpawnActorFromClass` "/Game/BP_class/BP_ElavatorOutside.BP_ElavatorOutside_C" (`KismetMathLibrary.MakeTransform` _returnvalue_location (`SceneComponent.K2_GetComponentRotation` (`self.Elavator`))) "Undefined" "MultiplyWithRoot" self self null))
        (set `/Game/BP_class/BP_ElavatorOutside.floor num` _index _returnvalue)))
    (:`then_1`
      ;[1 1 1] Build button
      (for _index_2 (range (`self.Number Of Floors`)) :!label _label
        (for _index_3 (range (`self.Col`))
          (bind _output_get (set `self.Count` (+ _count 1)))
          (if (<= _output_get (`self.Number Of Floors`))
            (bind _returnvalue_2 (`|SpawnActorFromClass` "/Game/BP_class/BP_Button.BP_Button_C" (`KismetMathLibrary.MakeTransform` (`KismetMathLibrary.MakeVector` _returnvalue_x_2 (+ (* _index_3 (`self.Distance`)) _returnvalue_y_2) (+ (* _index_2 (`self.Distance`)) _returnvalue_z)) (`SceneComponent.K2_GetComponentRotation` (`self.Button place`))) "Undefined" "MultiplyWithRoot" null (- _count 1) self null))
            (`SceneComponent.SetMobility` (`Actor.RootComponent` _returnvalue_2) "Movable")
            (`self.K2_AttachToComponent` _returnvalue_2 (`self.Elavator`) "Socket" "KeepWorld" "KeepWorld" "KeepWorld" true)
            (else
              (goto _label :!via `Break`)))))
      (set `self.Count` 0))))

(fn `UserConstructionScript`
  (bind _button_place (`self.Button place`))
  (bind (_relativelocation_x _relativelocation_y _relativelocation_z) (`KismetMathLibrary.BreakVector` (`SceneComponent.RelativeLocation` _button_place)))
  (`|ExecutionSequence`
    (:`then_0`
      ;[1 1 1] Building elavator outside
      (for _index (range (+ (`self.Number Of Floors`) 1))
        (`AddComponent|NODE_AddStaticMeshComponent-6` :`RelativeTransform` (`KismetMathLibrary.MakeTransform` (`KismetMathLibrary.Conv_IntVectorToVector` (make `IntVector` 0 0 (* _index (`self.Height of ElavatorOutside`))))))))
    (:`then_1`
      ;[1 1 1] Build button
      (for _index_2 (range (`self.Number Of Floors`)) :!label _label
        (for _index_3 (range (`self.Col`))
          (bind _output_get (set `self.Count` (+ (`self.Count`) 1)))
          (if (<= _output_get (`self.Number Of Floors`))
            (`AddComponent|NODE_AddStaticMeshComponent-9` :`RelativeTransform` (`KismetMathLibrary.MakeTransform` (`KismetMathLibrary.MakeVector` _relativelocation_x (- (* _index_3 (`self.Distance`)) _relativelocation_y) (+ (* _index_2 (`self.Distance`)) _relativelocation_z)) (`SceneComponent.RelativeRotation` _button_place) (0.028 0.028 0.028)))
            (else
              (goto _label :!via `Break`)))))
      (set `self.Count` 0))))